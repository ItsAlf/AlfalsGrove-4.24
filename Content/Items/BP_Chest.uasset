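; Interactable survival-mode chest that costs kills to open, spawning a random item from its pool once and deducting the kills from the game mode.
; On BeginPlay it may replace itself with a rare chest or mimic dispenser, otherwise scales its cost by difficulty.
; Opening spends the visuals and audio; too few kills plays a widget warning.
; A looping timer hides the cost nameplate when the player moves away.
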(event Custom|CheckNameplate
  (Utilities|Time|SetTimerbyEvent (delegate Custom|CheckNameplate) 1.5 true)
  (if (and (> (Transformation|GetDistanceTo (Variables|Default|GetPlayer_Ref)) 2e+02) (Rendering|IsVisible (Variables|Default|GetKillsNeeded)))
    (Rendering|SetVisibility (Variables|Default|GetKillsNeeded) false false)))

(event Custom|Update%20Cost
  (if (Variables|Default|GetShould_I_Update)
    _))

(event EventBeginPlay
  (bind _returnvalue (Math|Random|RandomFloatinRange 0.0 1e+02))
  (bind _box (Variables|Default|GetBox))
  (bind _returnvalue_2 (Transformation|GetWorldTransform _box))
  (bind _asgm_survival (Utilities|Casting|CastToGM_Survival (Game|GetGameMode)))
  (Variables|Default|SetGM_Ref _asgm_survival)
  (bind _asbp_player_character (Utilities|Casting|CastToBP_PlayerCharacter (Game|GetPlayerCharacter 0)))
  (Variables|Default|SetPlayer_Ref _asbp_player_character)
  (CallFunction|CheckNameplate)
  (if (Variables|Default|GetShould_I_Update)
    (if (>= (Math|Float|Truncate _returnvalue) 98)
      (Game|SpawnActorfromClass "/Game/Items/BP_RareChest.BP_RareChest_C" _returnvalue_2 "Undefined" 0 false 0)
      (Actor|DestroyActor)
      (elif (>= (Math|Float|Truncate _returnvalue) 96)
        (Game|SpawnActorfromClass "/Game/Enemies/BP_MimicDispenser.BP_MimicDispenser_C" _returnvalue_2 "Undefined" 0 0 0.5 false true 0 true 0)
        (Actor|DestroyActor)
        (else
          (Variables|Default|SetKillsToOpen (+ (Math|Float|Truncate (* (Variables|/Game/PlayerBlueprints/Blueprints/GM_Survival.GM_Survival_C|GetDifficultyMultiplier (Variables|Default|GetGM_Ref)) (Variables|Default|GetScalingCoefficient))) (Variables|Default|GetKillsToOpen))))))))

(event EventInteractInterface
  (bind _gm_ref (Variables|Default|GetGM_Ref))
  (bind _itempool (Variables|Default|GetItemPool))
  (bind _itemspawnpoint (Variables|Default|GetItemSpawnPoint))
  (bind _staticmesh (Variables|Default|GetStaticMesh))
  (bind _returnvalue (Transformation|GetWorldTransform _itemspawnpoint))
  (bind _asgm_survival (Utilities|Casting|CastToGM_Survival (Game|GetGameMode)))
  (if (>= (Variables|/Game/PlayerBlueprints/Blueprints/GM_Survival.GM_Survival_C|GetKills _asgm_survival) (Variables|Default|GetKillsToOpen))
    (Utilities|FlowControl|DoOnce false
      (:Completed
        (bind _returnvalue_2 (Game|SpawnActorfromClass (Utilities|Array|Get(acopy) _itempool (Math|Random|RandomIntegerinRange 0 (- (Utilities|Array|Length _itempool) 1))) _returnvalue "AlwaysSpawn" 0 5e+02 1.5e+03 true 0))
        (Development|PrintString (Utilities|GetDisplayName _returnvalue_2))
        (Audio|PlaySoundatLocation "/Game/Sounds/ItemSpawn_Cue.ItemSpawn_Cue" (.Location (Math|Transform|BreakTransform _returnvalue)) "0, 0, 0" 1.0 1.0 0.0 0 0 0)
        (Rendering|Components|Light|SetIntensity (Variables|Default|GetPointLight) 0.0)
        (Components|Activation|Deactivate (Variables|Default|GetNiagara))
        (Rendering|Material|SetMaterial _staticmesh 1 "/Game/Materials/M_Dispenser_Spent.M_Dispenser_Spent")
        (Rendering|Material|SetMaterial _staticmesh 2 "/Game/Materials/M_Dispenser_Spent.M_Dispenser_Spent")
        (Components|DestroyComponent (Variables|Default|GetSphere))
        (Variables|Default|SetOpened true)
        (Variables|/Game/PlayerBlueprints/Blueprints/GM_Survival.GM_Survival_C|SetKills _gm_ref (- (Variables|/Game/PlayerBlueprints/Blueprints/GM_Survival.GM_Survival_C|GetKills _gm_ref) (Variables|Default|GetKillsToOpen)))))
    (else
      (Development|PrintString "You need more kills!" true true "(R=0.133758,G=1.000000,B=0.000000,A=1.000000)" 4.0)
      (bind _askills_required (Utilities|Casting|CastToKillsRequired (UserInterface|GetUserWidgetObject (Variables|Default|GetKillsNeeded))))
      (UserInterface|Animation|PlayAnimation _askills_required (Variables|/Game/UI/KillsRequired.KillsRequired_C|GetNotEnough _askills_required) 0.0 1 "Forward" 1.0 false))))

(fn ConstructionScript)

(fn DisplayCost
  (bind _killsneeded (Variables|Default|GetKillsNeeded))
  (if (not (Variables|Default|GetOpened))
    (bind _askills_required (Utilities|Casting|CastToKillsRequired (UserInterface|GetUserWidgetObject _killsneeded)))
    (Variables|/Game/UI/KillsRequired.KillsRequired_C|SetChestRef _askills_required self)
    (Rendering|SetVisibility _killsneeded true false)))