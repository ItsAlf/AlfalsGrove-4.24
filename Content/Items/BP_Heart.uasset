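; BP_Heart is a heart pickup that adds its HeartWorth to the GM_Survival kill count.
; On spawn it pops upward with random drift, or destroys itself if over 700 hearts exist.
; After three seconds it clears Heal and removes its trail; 45 seconds later it triggers DoFunction itself.
; DoFunction runs once, updating the HUD counter, playing a sound, healing 5% max health if Heal remains set, then destroying the actor.
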(event EventBeginPlay
  (|CallParentFunction)
  (bind _outactors (Actor|GetAllActorsOfClass "BP_Heart_C"))
  (if (> (Utilities|Array|Length _outactors) 700)
    (Actor|DestroyActor)
    (else
      (Physics|AddImpulse (Variables|Default|GetSphere) (Math|Vector|MakeVector (Math|Random|RandomFloatinRange -25.0 25.0) (Math|Random|RandomFloatinRange -25.0 25.0) 1e+02) "None" true)
      (Utilities|FlowControl|Delay 3.0)
      (Variables|Default|SetHeal false)
      (Components|DestroyComponent (Variables|Default|GetTrails))
      (Utilities|FlowControl|Delay 45.0)
      (CallFunction|DoFunction))))

(event Collision|EventActorBeginOverlap
  (params (OtherActor :type Actor%20Object%20Reference)))

(event EventTick
  (params (DeltaSeconds :type Float%20%28single-precision%29)))

(event EventDoFunction
  (params (PlayerCharacter :type BP%20Player%20Character%20Object%20Reference) (Overlappedactor :type Actor%20Object%20Reference))
  (Utilities|FlowControl|DoOnce false
    (:Completed
      (bind _asgm_survival (Utilities|Casting|CastToGM_Survival (Game|GetGameMode)))
      (Variables|/Game/PlayerBlueprints/Blueprints/GM_Survival.GM_Survival_C|SetKills _asgm_survival (+ (Variables|/Game/PlayerBlueprints/Blueprints/GM_Survival.GM_Survival_C|GetKills _asgm_survival) (Variables|Default|GetHeartWorth)))
      (bind _asbp_player_character (Utilities|Casting|CastToBP_PlayerCharacter (Game|GetPlayerCharacter 0)))
      (Variables|Default|SetHealAmount (* (Variables|/Game/PlayerBlueprints/Blueprints/BP_PlayerCharacter.BP_PlayerCharacter_C|GetMaxHealth _asbp_player_character) 0.05))
      (Default|SomethingDied (Variables|/Game/UI/HUD.HUD_C|GetKillCounter (Variables|/Game/PlayerBlueprints/Blueprints/BP_PlayerCharacter.BP_PlayerCharacter_C|GetHUD_Ref _asbp_player_character)))
      (Audio|PlaySoundatLocation "/Game/Sounds/ItemPickup_Cue.ItemPickup_Cue" (Transformation|GetWorldLocation (Variables|Default|GetSphere)) "0, 0, 0" 1.0 1.0 0.0 0 0 0)
      (if (Variables|Default|GetHeal)
        (Default|Heal _asbp_player_character (Variables|Default|GetHealAmount)))
      (Utilities|FlowControl|Delay 0.2)
      (Actor|DestroyActor))))

(fn ConstructionScript
  (|CallParentFunction))