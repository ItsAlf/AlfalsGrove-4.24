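; Base pickup item that the player collects into their inventory on touching its sphere.
; When Magnetic is set, Tick pulls the sphere toward the player with impulses while within MagDistance.
; A DoOnce-gated overlap runs DoFunction, which stacks items by class or adds a slot, refreshes slots, adjusts stats, plays a sound, shows a HUD tooltip, then destroys the actor.
; The timed mesh rotation is disconnected.
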(event OnComponentBeginOverlap(Sphere)
  (params (OverlappedComponent :type Primitive%20Component%20Object%20Reference) (OtherActor :type Actor%20Object%20Reference) (OtherComp :type Primitive%20Component%20Object%20Reference) (OtherBodyIndex :type Integer) (bFromSweep :type Boolean) (SweepResult :type Hit%20Result%20Structure%20%28by%20ref%29))
  (if (Variables|Default|GetOnlyActivateOnPlayer)
    (bind _asbp_player_character (Utilities|Casting|CastToBP_PlayerCharacter OtherActor)))
  (Utilities|FlowControl|DoOnce false
    (:Completed
      (CallFunction|DoFunction _asbp_player_character OtherActor))))

(event Custom|BeginRoatation)

(event Custom|DoFunction
  (params (PlayerCharacter :type BP%20Player%20Character%20Object%20Reference) (Overlappedactor :type Actor%20Object%20Reference))
  (bind _collecteditems (Variables|/Game/PlayerBlueprints/Blueprints/BP_PlayerCharacter.BP_PlayerCharacter_C|GetCollectedItems PlayerCharacter))
  (bind _inventory (Variables|/Game/UI/CollectedItems.CollectedItems_C|GetInventory _collecteditems))
  (if (<= (Utilities|Array|Length _inventory) 0)
    (Utilities|Array|Add _inventory (Utilities|Struct|MakeS_SlotInfo (Variables|Default|GetItemStructure) 1))
    (Default|RefreshSlots _collecteditems (Variables|Default|GetItemStructure))
    (Default|AdjustStats (Variables|Default|GetPlayer_Ref) (Utilities|Struct|MakeS_SlotInfo (Variables|Default|GetItemStructure) 0))
    (else
      (for (_array_element _array_index) _inventory
        (if (== (.itemclass (.item _array_element)) (.itemclass (Variables|Default|GetItemStructure)))
          (Variables|Default|SetAddToStack true)
          (Variables|Default|SetTargetStack _array_index)
          (Variables|Default|SetStackQuantity (.quantity _array_element))))
      (if (Variables|Default|GetAddToStack)
        (Utilities|Array|SetArrayElem _inventory (Variables|Default|GetTargetStack) (Utilities|Struct|MakeS_SlotInfo (Variables|Default|GetItemStructure) (+ (Variables|Default|GetStackQuantity) 1)))
        (else
          (Utilities|Array|Add _inventory (Utilities|Struct|MakeS_SlotInfo (Variables|Default|GetItemStructure) 1))))
      (Default|RefreshSlots _collecteditems (Variables|Default|GetItemStructure))
      (Default|AdjustStats (Variables|Default|GetPlayer_Ref) (Utilities|Struct|MakeS_SlotInfo (Variables|Default|GetItemStructure) 0))))
  (Audio|PlaySoundatLocation "/Game/Sounds/ItemPickup_Cue.ItemPickup_Cue" (Transformation|GetWorldLocation (Variables|Default|GetSphere)) "0, 0, 0" 1.0 1.0 0.0 0 0 0)
  (Default|ShowTooltip (Variables|/Game/PlayerBlueprints/Blueprints/BP_PlayerCharacter.BP_PlayerCharacter_C|GetHUD_Ref (Variables|Default|GetPlayer_Ref)) (Variables|Default|GetItemStructure))
  (Utilities|FlowControl|Delay 0.2)
  (Actor|DestroyActor))

(event Custom|ResetTrigger
  (Utilities|FlowControl|DoOnce false) ; enters at Reset
)

(event EventBeginPlay
  (bind _asbp_player_character (Utilities|Casting|CastToBP_PlayerCharacter (Game|GetPlayerCharacter 0)))
  (Variables|Default|SetPlayer_Ref _asbp_player_character)
  (CallFunction|BeginRoatation))

(event EventTick
  (params (DeltaSeconds :type Float%20%28single-precision%29))
  (if (Variables|Default|GetMagnetic)
    (if (<= (Transformation|GetDistanceTo (Variables|Default|GetPlayer_Ref)) (Variables|Default|GetMagDistance))
      (Physics|AddImpulse (Variables|Default|GetSphere) (* (- (Transformation|GetActorLocation (Variables|Default|GetPlayer_Ref)) (Transformation|GetActorLocation)) (Variables|Default|GetMagPower)) "None" false))))

(fn ConstructionScript)

(fn TooltipAppear
  (bind _returnvalue (UserInterface|CreateWidget "/Game/UI/ItemPickupTooltip.ItemPickupTooltip_C" (Game|GetPlayerController 0) (Variables|Default|GetItemStructure)))
  (bind _returnvalue_2 (Class|CanvasPanel|AddChildtoCanvas (Variables|/Game/UI/HUD.HUD_C|GetCanvasPanel_0 (Variables|/Game/PlayerBlueprints/Blueprints/BP_PlayerCharacter.BP_PlayerCharacter_C|GetHUD_Ref (Variables|Default|GetPlayer_Ref))) _returnvalue))
  (Class|CanvasPanelSlot|SetAutoSize _returnvalue_2 true)
  (Class|CanvasPanelSlot|SetAnchors _returnvalue_2 (Utilities|Struct|MakeAnchors "(X=0.000000,Y=0.750000)" "(X=0.000000,Y=0.750000)"))
  (Class|CanvasPanelSlot|SetPosition _returnvalue_2 "(X=180.000000,Y=0.000000)")
  (return))