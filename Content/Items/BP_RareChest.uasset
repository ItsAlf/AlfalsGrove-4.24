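; Rare chest variant that spawns a BP_Guardian at BeginPlay and stays locked while that type of actor overlaps its sphere trigger.
; When unlocked, player overlap with the box runs the parent's interact logic, while the chest's own InteractInterface override is empty.
; DisplayCost briefly shows a locked indicator, or once unlocked destroys it and defers to the parent's cost display.
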(event OnComponentBeginOverlap(Sphere1)
  (params (OverlappedComponent :type Primitive%20Component%20Object%20Reference) (OtherActor :type Actor%20Object%20Reference) (OtherComp :type Primitive%20Component%20Object%20Reference) (OtherBodyIndex :type Integer) (bFromSweep :type Boolean) (SweepResult :type Hit%20Result%20Structure%20%28by%20ref%29))
  (Utilities|Casting|CastToBP_Guardian OtherActor)
  (Variables|Default|SetLocked true))

(event OnComponentEndOverlap(Sphere1)
  (params (OverlappedComponent :type Primitive%20Component%20Object%20Reference) (OtherActor :type Actor%20Object%20Reference) (OtherComp :type Primitive%20Component%20Object%20Reference) (OtherBodyIndex :type Integer))
  (Utilities|Casting|CastToBP_Guardian OtherActor)
  (Variables|Default|SetLocked false))

(event OnComponentBeginOverlap(Box)
  (params (OverlappedComponent :type Primitive%20Component%20Object%20Reference) (OtherActor :type Actor%20Object%20Reference) (OtherComp :type Primitive%20Component%20Object%20Reference) (OtherBodyIndex :type Integer) (bFromSweep :type Boolean) (SweepResult :type Hit%20Result%20Structure%20%28by%20ref%29))
  (Utilities|Casting|CastToBP_PlayerCharacter OtherActor)
  (if (not (Variables|Default|GetLocked))
    (|CallParentFunction)))

(event EventBeginPlay
  (Variables|Default|SetRareChest true)
  (Variables|Default|SetDestroyMe false)
  (Game|SpawnActorfromClass "/Game/Enemies/BP_Guardian.BP_Guardian_C" (Transformation|GetWorldTransform (Variables|Default|GetScene1)) "AdjustIfPossibleButAlwaysSpawn" 0 0 0.5 true false 0 false 0)
  (|CallParentFunction))

(event Collision|EventActorBeginOverlap
  (params (OtherActor :type Actor%20Object%20Reference)))

(event EventTick
  (params (DeltaSeconds :type Float%20%28single-precision%29)))

(event EventInteractInterface)

(event EventDisplayCost
  (bind _i_am_locked (Variables|Default|GetI_Am_Locked))
  (bind _i_am_locked_2 (Variables|Default|GetI_Am_Locked))
  (if (Variables|Default|GetLocked)
    (Utilities|IsValid _i_am_locked
      (:Is%20Valid
        (Rendering|SetVisibility _i_am_locked true false)
        (Utilities|FlowControl|Delay 3.0)
        (Utilities|IsValid _i_am_locked
          (:Is%20Valid
            (Rendering|SetVisibility _i_am_locked false false)))))
    (else
      (Utilities|IsValid _i_am_locked_2
        (:Is%20Valid
          (Components|DestroyComponent _i_am_locked_2))
        (:Is%20Not%20Valid
          _))
      (|CallParentFunction))))

(fn ConstructionScript
  (|CallParentFunction))