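; BP_Damage is an item that damages what overlaps it through DoFunction, then destroys itself.
; With a valid instigator, it ignores that instigator by resetting the trigger and hits others using the BP_TurtleDropper's DamageIDo.
; Without one, it resets on non-Characters and takes DamageIDo from a BP_TurtleDropper owner.
; The fixed-damage fallback passes the overlapped actor as causer, with no damaged actor set.
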(event EventBeginPlay
  (|CallParentFunction) ; This node is disabled and will not be called.\nDrag off pins to build functionality.
)

(event Collision|EventActorBeginOverlap
  (params (OtherActor :type Actor%20Object%20Reference)))

(event EventTick
  (params (DeltaSeconds :type Float%20%28single-precision%29))
  (|CallParentFunction DeltaSeconds) ; This node is disabled and will not be called.\nDrag off pins to build functionality.
)

(event EventDoFunction
  (params (PlayerCharacter :type BP%20Player%20Character%20Object%20Reference) (Overlappedactor :type Actor%20Object%20Reference))
  (bind _returnvalue (Game|GetInstigator))
  (if (Utilities|IsValid _returnvalue)
    (if (== Overlappedactor _returnvalue)
      (CallFunction|ResetTrigger :!label _label)
      (else
        (bind _asbp_turtle_dropper (Utilities|Casting|CastToBP_TurtleDropper _returnvalue))
        (Game|Damage|ApplyDamage Overlappedactor (Variables|/Game/Enemies/BP_Enemy_Parent.BP_Enemy_Parent_C|GetDamageIDo _asbp_turtle_dropper) (Pawn|GetController _returnvalue) _returnvalue)
        (Actor|DestroyActor :!label _label_2)))
    (else
      (Utilities|Casting|CastToCharacter Overlappedactor
        (:then
          (bind _asbp_turtle_dropper_2 (Utilities|Casting|CastToBP_TurtleDropper (Components|GetOwner))
            (:then
              (Game|Damage|ApplyDamage Overlappedactor (Variables|/Game/Enemies/BP_Enemy_Parent.BP_Enemy_Parent_C|GetDamageIDo _asbp_turtle_dropper_2) 0 0)
              (goto _label_2))
            (:CastFailed
              (Game|Damage|ApplyDamage 0 1e+01 0 Overlappedactor)
              (goto _label_2))))
        (:CastFailed
          (goto _label))))))

(fn ConstructionScript
  (|CallParentFunction))