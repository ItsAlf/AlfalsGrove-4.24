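; Base projectile actor that configures speed, size, collision and optional homing on an enemy or player target at BeginPlay.
; Overlaps apply damage once to non-owners; player hits on enemies spawn hit particles, and crits trigger a point-blank heal and end the projectile.
; Blocking hits or a lifetime timer also call Die, which spawns a configurable explosion, hides the projectile, then destroys it after a short delay.
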(event Custom|Timer%20Till%20Death
  (Utilities|FlowControl|Delay 25.0)
  (Utilities|Die))

(fn ConstructionScript)

(fn FindHomingTarget
  (params (Target :type Actor%20Object%20Reference))
  (Utilities|IsValid Target
    (:Is%20Valid
      (bind _asbp_enemy_parent (Utilities|Casting|CastToBP_Enemy_Parent Target)
        (:then
          (if (< (Math|Vector|VectorLength (- (Transformation|GetActorLocation) (Transformation|GetActorLocation _asbp_enemy_parent))) (LocalVariables|GetClosestDistance))
            (LocalVariables|SetClosestDistance (Math|Vector|VectorLength (- (Transformation|GetActorLocation) (Transformation|GetActorLocation _asbp_enemy_parent))))
            (return (Variables|/Script/Engine.Character|GetCapsuleComponent _asbp_enemy_parent))))
        (:CastFailed
          (bind _asbp_player_character (Utilities|Casting|CastToBP_PlayerCharacter Target))
          (if (< (Math|Vector|VectorLength (- (Transformation|GetActorLocation) (Transformation|GetActorLocation _asbp_player_character))) (LocalVariables|GetClosestDistance))
            (LocalVariables|SetClosestDistance (Math|Vector|VectorLength (- (Transformation|GetActorLocation) (Transformation|GetActorLocation _asbp_player_character))))
            (return (Variables|/Script/Engine.Character|GetCapsuleComponent _asbp_player_character))))))))

(fn DamageHitActor
  (params (OverlapActor :type Actor%20Object%20Reference) (Hit :type Hit%20Result%20Structure%20%28by%20ref%29))
  (bind _returnvalue (Game|GetInstigatorController))
  (bind _myowner (Variables|Default|GetMyOwner))
  (bind _mydamagetype (Variables|Default|GetMyDamageType))
  (Variables|Default|SetOverlapActor OverlapActor)
  (if (and (!= _myowner OverlapActor) (!= _myowner OverlapActor))
    (Utilities|FlowControl|DoOnce false
      (:Completed
        (Utilities|IsValid _returnvalue
          (:Is%20Valid
            (Game|Damage|ApplyDamage (Variables|Default|GetOverlapActor) (Variables|Default|GetDamage) _returnvalue (Game|GetInstigator) _mydamagetype))
          (:Is%20Not%20Valid
            (Game|Damage|ApplyDamage 0 0.0 0 0 _mydamagetype)))
        (Utilities|Casting|CastToBP_Enemy_Parent (Variables|Default|GetOverlapActor))
        (bind _asbp_player_character (Utilities|Casting|CastToBP_PlayerCharacter (Game|GetInstigator)))
        (Game|SpawnActorfromClass "/Game/Projectiles/HitParticles.HitParticles_C" (Math|Conversions|ToTransform(Vector) (.Location (Collision|BreakHitResult Hit))) "Undefined" 0 0)
        (if (== (Variables|Default|GetMyDamageType) "/Game/DamageTypes/CritDamage.CritDamage_C")
          (Default|PointBlankHeal _asbp_player_character)
          (return true))))
    (else
      (return false))))

(event OnComponentHit(Sphere)
  (params (HitComponent :type Primitive%20Component%20Object%20Reference) (OtherActor :type Actor%20Object%20Reference) (OtherComp :type Primitive%20Component%20Object%20Reference) (NormalImpulse :type Vector :default "0, 0, 0") (Hit :type Hit%20Result%20Structure%20%28by%20ref%29))
  (if (Variables|Default|GetDebugMode)
    (Development|PrintString (Utilities|GetDisplayName OtherActor)))
  (Utilities|Die))

(event OnComponentBeginOverlap(Sphere)
  (params (OverlappedComponent :type Primitive%20Component%20Object%20Reference) (OtherActor :type Actor%20Object%20Reference) (OtherComp :type Primitive%20Component%20Object%20Reference) (OtherBodyIndex :type Integer) (bFromSweep :type Boolean) (SweepResult :type Hit%20Result%20Structure%20%28by%20ref%29))
  (bind _success (CallFunction|DamageHitActor OtherActor SweepResult))
  (if _success
    (Utilities|Die)))

(event EventBeginPlay
  (bind _projectilemovement (Variables|Default|GetProjectileMovement))
  (bind _projectilemovement_2 (Variables|Default|GetProjectileMovement))
  (bind _sphere (Variables|Default|GetSphere))
  (bind _sphere_2 (Variables|Default|GetSphere))
  (bind _myspeed (Variables|Default|GetMySpeed))
  (bind _returnvalue (Transformation|GetWorldTransform _sphere_2))
  (if (Variables|Default|GetPRojectileCollisions)
    _
    (else
      (Collision|SetCollisionResponsetoChannel (Variables|Default|GetSphere) "ECC_GameTraceChannel1" "ECR_Ignore")))
  (if (Variables|Default|GetGoThruAll)
    (Collision|SetCollisionResponsetoChannel _sphere "ECC_WorldStatic" "ECR_Ignore")
    (Collision|SetCollisionResponsetoChannel _sphere "ECC_WorldDynamic" "ECR_Ignore"))
  (bind _output_get (Variables|/Script/Engine.ProjectileMovementComponent|SetbIsHomingProjectile _projectilemovement_2 (Variables|Default|GetIsHoming)))
  (if _output_get
    (Variables|/Script/Engine.ProjectileMovementComponent|SetHomingAccelerationMagnitude _projectilemovement_2 (Variables|Default|GetHomingPower))
    (bind _truetarget (CallFunction|FindHomingTarget (Variables|Default|GetHomingTarget)))
    (Variables|/Script/Engine.ProjectileMovementComponent|SetHomingTargetComponent _projectilemovement_2 _truetarget))
  (Variables|Default|SetExplosionDamageToDo (Variables|Default|GetExplosionDamage))
  (Variables|Default|SetSizeOfExplosion (Variables|Default|GetExplosionSize))
  (CallFunction|TimerTillDeath)
  (Variables|Default|SetPlayer_Ref (.AsBP%20Player%20Character (Utilities|Casting|CastToBP_PlayerCharacter (Game|GetPlayerCharacter 0))))
  (Variables|/Script/Engine.ProjectileMovementComponent|SetInitialSpeed _projectilemovement _myspeed)
  (Variables|/Script/Engine.ProjectileMovementComponent|SetMaxSpeed _projectilemovement _myspeed)
  (Transformation|SetWorldTransform _sphere_2 (Math|Transform|MakeTransform (.location _returnvalue) (.rotation _returnvalue) (Variables|Default|GetSize)) false false)
  (if (== (Game|GetInstigator) (Variables|Default|GetPlayer_Ref))
    (Variables|Default|SetStunHitActor (Variables|/Game/PlayerBlueprints/Blueprints/BP_PlayerCharacter.BP_PlayerCharacter_C|GetPointBlank (Variables|Default|GetPlayer_Ref)))))