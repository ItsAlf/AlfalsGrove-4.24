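; Survival game mode that runs escalating enemy waves and owns the player's saved progress.
; Looping timers raise difficulty, shifting spawn odds toward rarer pools, and spawn enemies at random points while under a population cap.
; Chests respawn at BeginPlay and on forced difficulty increases.
; Helper functions persist graphics settings, skins, run stats, item unlocks and last location in SaveGame slots, applying graphics via console commands and showing unlock notifications.
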(fn ConstructionScript)

(fn SpawnEnemies
  (bind _usedpoints (Variables|Default|GetUsedPoints))
  ;[1 1 1] Ensure we're not at enemy limit
  (bind _outactors (Actor|GetAllActorsOfClass "/Game/Enemies/BP_Enemy_Parent.BP_Enemy_Parent_C"))
  (if (< (Utilities|Array|Length _outactors) 100)
    (bind _outactors_2 (Actor|GetAllActorsOfClass "/Game/LevelPrototypingTools/BP_EnemySpawnPoint.BP_EnemySpawnPoint_C"))
    (bind _output_get (Variables|Default|SetSpawnPoints _outactors_2))
    (for _array_element _output_get
      (if (Default|CheckShouldSpawn _array_element)
        (Utilities|FlowControl|DoN (Math|Random|RandomIntegerinRange (Math|Integer|Clamp(Integer) (- (Utilities|Array|Length _output_get) 10) 0 5) (- (Utilities|Array|Length _output_get) 1))
          (:Exit
            (bind _output_get_2 (Variables|Default|SetCurrentPoint (Math|Random|RandomIntegerinRange 0 (- (Utilities|Array|Length (Variables|Default|GetSpawnPoints)) 1))))
            (if (not (Utilities|Array|ContainsItem _usedpoints _output_get_2))
              (Utilities|Array|Add _usedpoints (Variables|Default|GetCurrentPoint))
              (if (not (Variables|/Game/LevelPrototypingTools/BP_EnemySpawnPoint.BP_EnemySpawnPoint_C|GetSpawnedCharacter (Utilities|Array|Get(acopy) (Variables|Default|GetSpawnPoints) (Variables|Default|GetCurrentPoint))))
                (LocalVariables|SetPoolRoll (Math|Random|RandomFloatinRange 0.0 1e+02))
                (if (Math|Float|InRange(Float) (Math|Conversions|ToFloat(Integer) (Math|Float|Truncate (LocalVariables|GetPoolRoll))) 0.0 (Variables|Default|GetCommonChance))
                  (Development|PrintString "COMMON POOL")
                  (Variables|Default|SetPoolToUse (Variables|Default|GetCommonSpawnPool))
                  (bind _returnvalue (Game|SpawnActorfromClass (Utilities|Array|Get(acopy) (Variables|Default|GetPoolToUse) (Math|Random|RandomIntegerinRange 0 (- (Utilities|Array|Length (Variables|Default|GetPoolToUse)) 1))) (Transformation|GetWorldTransform (Variables|/Script/Engine.Actor|GetRootComponent (Utilities|Array|Get(acopy) (Variables|Default|GetSpawnPoints) (Variables|Default|GetCurrentPoint)))) "Undefined" 0 0 0.5 true false 0 true 0 :!label _label))
                  (Utilities|Array|Add (Variables|Default|GetEnemiesSpawned) _returnvalue)
                  (Audio|PlaySoundatLocation "/Game/Sounds/EnemySpawn_Cue.EnemySpawn_Cue" (.Location (Math|Transform|BreakTransform (Transformation|GetWorldTransform (Variables|/Script/Engine.Actor|GetRootComponent (Utilities|Array|Get(acopy) (Variables|Default|GetSpawnPoints) (Variables|Default|GetCurrentPoint)))))) "0, 0, 0" 1.0 1.0 0.0 0 0 0)
                  (Variables|/Game/LevelPrototypingTools/BP_EnemySpawnPoint.BP_EnemySpawnPoint_C|SetSpawnedCharacter (Utilities|Array|Get(acopy) (Variables|Default|GetSpawnPoints) (Variables|Default|GetCurrentPoint)) true)
                  (elif (Math|Float|InRange(Float) (Math|Conversions|ToFloat(Integer) (Math|Float|Truncate (LocalVariables|GetPoolRoll))) (Variables|Default|GetCommonChance) (Variables|Default|GetRareLowerLimit) false)
                    (Development|PrintString "UNCOMMON POOL")
                    (Variables|Default|SetPoolToUse (Variables|Default|GetUncommonSpawnPool))
                    (goto _label)
                    (elif (Math|Float|InRange(Float) (Math|Conversions|ToFloat(Integer) (Math|Float|Truncate (LocalVariables|GetPoolRoll))) (Variables|Default|GetRareLowerLimit) 1e+02 false)
                      (Development|PrintString "RARE POOL")
                      (Variables|Default|SetPoolToUse (Variables|Default|GetRareSpawnPool))
                      (goto _label)
                      (else
                        (Development|PrintString (Utilities|String|ToString(Integer) (Math|Float|Truncate (LocalVariables|GetPoolRoll))))))))))))))
    ;[1 1 1] Reset
    (for _array_element_2 (Variables|Default|GetSpawnPoints)
      (Variables|/Game/LevelPrototypingTools/BP_EnemySpawnPoint.BP_EnemySpawnPoint_C|SetSpawnedCharacter _array_element_2 false)
      (Utilities|Array|Clear (Variables|Default|GetUsedPoints)))))

(fn SpawnChests
  (bind _usedpoints (Variables|Default|GetUsedPoints))
  (bind _outactors (Actor|GetAllActorsOfClass "/Game/Items/BP_Chest.BP_Chest_C"))
  (for _array_element _outactors
    (if (Variables|/Game/Items/BP_Chest.BP_Chest_C|GetDestroyMe _array_element)
      (Actor|DestroyActor _array_element :!label _label)
      (elif (Variables|/Game/Items/BP_Chest.BP_Chest_C|GetOpened _array_element)
        (goto _label))))
  (bind _outactors_2 (Actor|GetAllActorsOfClass "/Game/LevelPrototypingTools/BP_ChestSpawnPoint.BP_ChestSpawnPoint_C"))
  (for _array_element_2 _outactors_2
    (Utilities|FlowControl|DoN (Math|Random|RandomIntegerinRange 2 (- (Utilities|Array|Length _outactors_2) 1))
      (:Exit
        (bind _outactors_3 (Actor|GetAllActorsOfClass "/Game/LevelPrototypingTools/BP_ChestSpawnPoint.BP_ChestSpawnPoint_C"))
        (bind _output_get (Variables|Default|SetCurrentPoint (Math|Random|RandomIntegerinRange 0 (- (Utilities|Array|Length _outactors_3) 1))))
        (if (not (Utilities|Array|ContainsItem _usedpoints _output_get))
          (Utilities|Array|Add _usedpoints (Variables|Default|GetCurrentPoint))
          (if (not (Variables|/Game/LevelPrototypingTools/BP_ChestSpawnPoint.BP_ChestSpawnPoint_C|GetSpawnedChest (Utilities|Array|Get(acopy) _outactors_3 (Variables|Default|GetCurrentPoint))))
            (Game|SpawnActorfromClass "/Game/Items/BP_Chest.BP_Chest_C" (Transformation|GetWorldTransform (Variables|/Game/LevelPrototypingTools/BP_ChestSpawnPoint.BP_ChestSpawnPoint_C|GetScene (Utilities|Array|Get(acopy) _outactors_3 (Variables|Default|GetCurrentPoint)))) "AdjustIfPossibleButAlwaysSpawn" 0 true 0)
            (Variables|/Game/LevelPrototypingTools/BP_ChestSpawnPoint.BP_ChestSpawnPoint_C|SetSpawnedChest (Utilities|Array|Get(acopy) _outactors_3 (Variables|Default|GetCurrentPoint)) true)
            (Actor|DestroyActor _array_element_2)))))))

(fn SaveGraphics
  (params (PP_Index :type Integer) (AA_Index :type Integer) (SQ_Index :type Integer) (FPS_Index :type Integer) (GraphicalIndex :type Integer) (GameSkin1 :type Integer) (UnlockedSkins :type Array%20of%20Texts) (LookSensitivity :type Float%20%28single-precision%29))
  (bind _returnvalue (SaveGame|CreateSaveGameObject "/Game/PlayerBlueprints/Blueprints/Saves/GraphicsSaves.GraphicsSaves_C"))
  (Variables|/Game/PlayerBlueprints/Blueprints/Saves/GraphicsSaves.GraphicsSaves_C|SetPP_Index _returnvalue PP_Index)
  (Variables|/Game/PlayerBlueprints/Blueprints/Saves/GraphicsSaves.GraphicsSaves_C|SetAA_Index _returnvalue AA_Index)
  (Variables|/Game/PlayerBlueprints/Blueprints/Saves/GraphicsSaves.GraphicsSaves_C|SetSQ_Index _returnvalue SQ_Index)
  (Variables|/Game/PlayerBlueprints/Blueprints/Saves/GraphicsSaves.GraphicsSaves_C|SetFPS_Index _returnvalue FPS_Index)
  (Variables|/Game/PlayerBlueprints/Blueprints/Saves/GraphicsSaves.GraphicsSaves_C|SetGraphicalIndex _returnvalue GraphicalIndex)
  (Variables|/Game/PlayerBlueprints/Blueprints/Saves/GraphicsSaves.GraphicsSaves_C|SetGameSkin _returnvalue GameSkin1)
  (Variables|/Game/PlayerBlueprints/Blueprints/Saves/GraphicsSaves.GraphicsSaves_C|SetUnlockedSkins _returnvalue UnlockedSkins)
  (Variables|/Game/PlayerBlueprints/Blueprints/Saves/GraphicsSaves.GraphicsSaves_C|SetLookSensitivity _returnvalue LookSensitivity)
  (SaveGame|SaveGametoSlot _returnvalue "Graphics")
  (return))

(fn LoadGraphics
  (params (SetGraphics :type Boolean))
  (bind _returnvalue (SaveGame|LoadGamefromSlot "Graphics"))
  (bind _asgraphics_saves (Utilities|Casting|CastToGraphicsSaves _returnvalue))
  (if SetGraphics
    (bind _output_get (LocalVariables|SetAA_Index (Variables|/Game/PlayerBlueprints/Blueprints/Saves/GraphicsSaves.GraphicsSaves_C|GetAA_Index _asgraphics_saves)))
    (bind _output_get_2 (LocalVariables|SetPP_Index (Variables|/Game/PlayerBlueprints/Blueprints/Saves/GraphicsSaves.GraphicsSaves_C|GetPP_Index _asgraphics_saves)))
    (bind _output_get_3 (LocalVariables|SetFPS_Index (Variables|/Game/PlayerBlueprints/Blueprints/Saves/GraphicsSaves.GraphicsSaves_C|GetFPS_Index _asgraphics_saves)))
    (bind _output_get_4 (LocalVariables|SetSQ_Index (Variables|/Game/PlayerBlueprints/Blueprints/Saves/GraphicsSaves.GraphicsSaves_C|GetSQ_Index _asgraphics_saves)))
    (bind _output_get_5 (LocalVariables|SetGraphicalIndex (Variables|/Game/PlayerBlueprints/Blueprints/Saves/GraphicsSaves.GraphicsSaves_C|GetGraphicalIndex _asgraphics_saves)))
    (for (_array_element _array_index) (Utilities|Array|MakeArray _output_get _output_get_2 _output_get_3 _output_get_4 _output_get_5)
      (CallFunction|ChangeGraphicSetting (Utilities|Select :Index _array_index :Option%200 (Variables|Default|GetAA_Commands) :Option%201 (Variables|Default|GetPP_Commands) :Option%202 (Variables|Default|GetFPS_Commands) :Option%203 (Variables|Default|GetSQ_Commands) :Option%204 (Variables|Default|GetResolutionCommands)) _array_element))
    (bind _asbp_player_character (Utilities|Casting|CastToBP_PlayerCharacter (Game|GetPlayerCharacter 0)))
    (Variables|/Game/PlayerBlueprints/Blueprints/BP_PlayerCharacter.BP_PlayerCharacter_C|SetLookSensitivity _asbp_player_character (Math|Float|Clamp(Float) (Variables|/Game/PlayerBlueprints/Blueprints/Saves/GraphicsSaves.GraphicsSaves_C|GetLookSensitivity _asgraphics_saves) 0.4))
    (bind _returnvalue_2 (SaveGame|DoesSaveGameExist "ItemUnlocks"))
    (if _returnvalue_2
      (bind _returnvalue_3 (SaveGame|LoadGamefromSlot "ItemUnlocks"))
      (bind _asitem_unlocks (Utilities|Casting|CastToItemUnlocks _returnvalue_3))
      (Variables|Default|SetRareItemPool (Variables|/Game/PlayerBlueprints/Blueprints/Saves/ItemUnlocks.ItemUnlocks_C|GetRareItemsUnlocked _asitem_unlocks))
      (Variables|Default|SetCommonItemPool (Variables|/Game/PlayerBlueprints/Blueprints/Saves/ItemUnlocks.ItemUnlocks_C|GetCommonItemsUnlocked _asitem_unlocks))
      (return (LocalVariables|GetAA_Index) (LocalVariables|GetPP_Index) (LocalVariables|GetFPS_Index) (LocalVariables|GetSQ_Index) (LocalVariables|GetGraphicalIndex) (Variables|/Game/PlayerBlueprints/Blueprints/Saves/GraphicsSaves.GraphicsSaves_C|GetUnlockedSkins _asgraphics_saves)))
    (else
      (return (Variables|/Game/PlayerBlueprints/Blueprints/Saves/GraphicsSaves.GraphicsSaves_C|GetAA_Index _asgraphics_saves) (Variables|/Game/PlayerBlueprints/Blueprints/Saves/GraphicsSaves.GraphicsSaves_C|GetPP_Index _asgraphics_saves) (Variables|/Game/PlayerBlueprints/Blueprints/Saves/GraphicsSaves.GraphicsSaves_C|GetFPS_Index _asgraphics_saves) (Variables|/Game/PlayerBlueprints/Blueprints/Saves/GraphicsSaves.GraphicsSaves_C|GetSQ_Index _asgraphics_saves) (Variables|/Game/PlayerBlueprints/Blueprints/Saves/GraphicsSaves.GraphicsSaves_C|GetGraphicalIndex _asgraphics_saves) (Variables|/Game/PlayerBlueprints/Blueprints/Saves/GraphicsSaves.GraphicsSaves_C|GetUnlockedSkins _asgraphics_saves)))))

(fn SaveUnlocks
  (params (CommonItemPool :type Array%20of%20BP%20Item%20Parent%20Class%20References) (RareItemPool :type Array%20of%20BP%20Item%20Parent%20Class%20References))
  (bind _returnvalue (SaveGame|DoesSaveGameExist "ItemUnlocks"))
  (if _returnvalue
    (bind _returnvalue_2 (SaveGame|LoadGamefromSlot "ItemUnlocks"))
    (bind _asitem_unlocks (Utilities|Casting|CastToItemUnlocks _returnvalue_2))
    (Variables|/Game/PlayerBlueprints/Blueprints/Saves/ItemUnlocks.ItemUnlocks_C|SetRareItemsUnlocked _asitem_unlocks RareItemPool)
    (Variables|/Game/PlayerBlueprints/Blueprints/Saves/ItemUnlocks.ItemUnlocks_C|SetCommonItemsUnlocked _asitem_unlocks CommonItemPool)
    (bind _returnvalue_3 (SaveGame|SaveGametoSlot _asitem_unlocks "ItemUnlocks"))
    (return _returnvalue_3)
    (else
      (bind _returnvalue_4 (SaveGame|CreateSaveGameObject "/Game/PlayerBlueprints/Blueprints/Saves/ItemUnlocks.ItemUnlocks_C"))
      (Variables|/Game/PlayerBlueprints/Blueprints/Saves/ItemUnlocks.ItemUnlocks_C|SetRareItemsUnlocked _returnvalue_4 RareItemPool)
      (Variables|/Game/PlayerBlueprints/Blueprints/Saves/ItemUnlocks.ItemUnlocks_C|SetCommonItemsUnlocked _returnvalue_4 CommonItemPool)
      (bind _returnvalue_5 (SaveGame|SaveGametoSlot _returnvalue_4 "ItemUnlocks"))
      (return _returnvalue_5))))

(fn ChangeGraphicSetting
  (params (Array :type Array%20of%20Texts) (Index :type Integer))
  (Development|ExecuteConsoleCommand (Utilities|String|ToString(Text) (Utilities|Array|Get(acopy) Array Index)) 0)
  (return))

(fn SavePlayerStats
  (params (LoadersUsed1 :type Integer) (Deaths1 :type Integer) (DamageDealt1 :type Float%20%28single-precision%29) (EnemiesDashed1 :type Integer) (EnemiesKilledPB1 :type Integer))
  (LocalVariables|SetLoadersUsed LoadersUsed1)
  (LocalVariables|SetDeaths Deaths1)
  (LocalVariables|SetDamageDealt DamageDealt1)
  (LocalVariables|SetEnemiesDashed EnemiesDashed1)
  (LocalVariables|SetEnemiesKilledPB EnemiesKilledPB1)
  (bind _returnvalue (SaveGame|DoesSaveGameExist "PlayerStats"))
  (if _returnvalue
    (bind _returnvalue_2 (SaveGame|LoadGamefromSlot "PlayerStats"))
    (bind _asplayer_stat_save (Utilities|Casting|CastToPlayerStatSave _returnvalue_2))
    (Default|AddtoTotalLoadersUsed _asplayer_stat_save (LocalVariables|GetLoadersUsed))
    (Default|AddtoAllTimeDeaths _asplayer_stat_save (LocalVariables|GetDeaths))
    (Default|AddtoEnemiesDashed _asplayer_stat_save (LocalVariables|GetEnemiesDashed))
    (Default|AddtoEnemiesKilledPB _asplayer_stat_save (LocalVariables|GetEnemiesKilledPB))
    (bind _newrecord (Default|SetDamageRecord _asplayer_stat_save (LocalVariables|GetDamageDealt) (Variables|/Game/PlayerBlueprints/Blueprints/Saves/PlayerStatSave.PlayerStatSave_C|GetDamageRecord _asplayer_stat_save)))
    (Development|PrintString "Player Stats Updated")
    (if _newrecord
      (Development|PrintString "New Record!")
      (return true)
      (else
        (return false)))
    (else
      (bind _returnvalue_3 (SaveGame|CreateSaveGameObject "/Game/PlayerBlueprints/Blueprints/Saves/PlayerStatSave.PlayerStatSave_C"))
      (Default|AddtoTotalLoadersUsed _returnvalue_3 (LocalVariables|GetLoadersUsed))
      (Default|AddtoAllTimeDeaths _returnvalue_3 (LocalVariables|GetDeaths))
      (Default|AddtoEnemiesDashed _returnvalue_3 (LocalVariables|GetEnemiesDashed))
      (Default|AddtoEnemiesKilledPB _returnvalue_3 (LocalVariables|GetEnemiesKilledPB))
      (Default|SetDamageRecord _returnvalue_3 (LocalVariables|GetDamageDealt) 0.0)
      (SaveGame|SaveGametoSlot _returnvalue_3 "PlayerStats")
      (Development|PrintString "Player Stats Created")
      (return true))))

(fn LoadPlayerStats
  (bind _returnvalue (SaveGame|DoesSaveGameExist "PlayerStats"))
  (if _returnvalue
    (bind _returnvalue_2 (SaveGame|LoadGamefromSlot "PlayerStats"))
    (bind _asplayer_stat_save (Utilities|Casting|CastToPlayerStatSave _returnvalue_2))
    (return (Variables|/Game/PlayerBlueprints/Blueprints/Saves/PlayerStatSave.PlayerStatSave_C|GetAllTimeDeaths _asplayer_stat_save) (Variables|/Game/PlayerBlueprints/Blueprints/Saves/PlayerStatSave.PlayerStatSave_C|GetDamageRecord _asplayer_stat_save) (Variables|/Game/PlayerBlueprints/Blueprints/Saves/PlayerStatSave.PlayerStatSave_C|GetEnemiesDashedInto _asplayer_stat_save) (Variables|/Game/PlayerBlueprints/Blueprints/Saves/PlayerStatSave.PlayerStatSave_C|GetEnemiesKilledPB _asplayer_stat_save) (Variables|/Game/PlayerBlueprints/Blueprints/Saves/PlayerStatSave.PlayerStatSave_C|GetTotalLoadersUsed _asplayer_stat_save) true)
    (else
      (Development|PrintString "No PlayerStats save"))))

(fn UnlockItem
  (params (ItemUnlocked :type BP%20Item%20Parent%20Class%20Reference) (UnlockName :type Name) (UnlockDesc :type Text))
  (Development|PrintString "unlocked!" true true "(R=0.000000,G=1.000000,B=0.223963,A=1.000000)")
  (Development|PrintString (Utilities|GetClassDisplayName ItemUnlocked) true true "(R=0.000000,G=1.000000,B=0.223963,A=1.000000)")
  (bind _array_element (Utilities|Array|ForEachLoopwithBreak (Variables|Default|GetAllCommonItems) :!label _label)
    (:LoopBody
      (bind _output_get (LocalVariables|SetCommonItem (== _array_element ItemUnlocked)))
      (if _output_get
        (goto _label Break)))
    (:Completed
      (if (LocalVariables|GetCommonItem)
        (Utilities|Array|Add (Variables|Default|GetCommonItemPool) ItemUnlocked)
        (else
          (Utilities|Array|Add (Variables|Default|GetRareItemPool) ItemUnlocked)))
      (CallFunction|SaveUnlocks (Variables|Default|GetCommonItemPool) (Variables|Default|GetRareItemPool))
      (CallFunction|UnlockNotification (Utilities|Struct|MakeAchievmentStructure UnlockName UnlockDesc (.ItemStructure (Utilities|GetClassDefaults ItemUnlocked)))))))

(fn CheckUnlockedItems
  (bind _returnvalue (SaveGame|DoesSaveGameExist "ItemUnlocks"))
  (if _returnvalue
    (bind _returnvalue_2 (SaveGame|LoadGamefromSlot "ItemUnlocks"))
    (bind _asitem_unlocks (Utilities|Casting|CastToItemUnlocks _returnvalue_2))
    (return (Variables|/Game/PlayerBlueprints/Blueprints/Saves/ItemUnlocks.ItemUnlocks_C|GetCommonItemsUnlocked _asitem_unlocks) (Variables|/Game/PlayerBlueprints/Blueprints/Saves/ItemUnlocks.ItemUnlocks_C|GetRareItemsUnlocked _asitem_unlocks) true)
    (else
      (Development|PrintString "No Save")
      (return (Variables|Default|GetCommonItemPool) (Variables|Default|GetRareItemPool) false))))

(fn UnlockNotification
  (params (Information :type Achievment%20Structure%20Structure))
  (bind _asbp_player_character (Utilities|Casting|CastToBP_PlayerCharacter (Game|GetPlayerCharacter 0)))
  (bind _returnvalue (UserInterface|CreateWidget "/Game/UI/Achievment.Achievment_C" (Game|GetPlayerController 0) Information))
  (bind _returnvalue_2 (Class|CanvasPanel|AddChildtoCanvas (Variables|/Game/UI/HUD.HUD_C|GetCanvasPanel_0 (Variables|/Game/PlayerBlueprints/Blueprints/BP_PlayerCharacter.BP_PlayerCharacter_C|GetHUD_Ref _asbp_player_character)) _returnvalue))
  (Class|CanvasPanelSlot|SetAutoSize _returnvalue_2 true)
  (Class|CanvasPanelSlot|SetAnchors _returnvalue_2 (Utilities|Struct|MakeAnchors "(X=0.500000,Y=0.100000)" "(X=0.500000,Y=0.100000)"))
  (Class|CanvasPanelSlot|SetPosition _returnvalue_2 "(X=-960.000000,Y=0.000000)")
  (return))

(fn UpdateUnlockedSkins
  (params (SkinToAdd :type Text%20%28by%20ref%29))
  (bind _returnvalue (SaveGame|DoesSaveGameExist "Graphics"))
  (if _returnvalue
    (bind _returnvalue_2 (SaveGame|LoadGamefromSlot "Graphics"))
    (bind _asgraphics_saves (Utilities|Casting|CastToGraphicsSaves _returnvalue_2))
    (bind _output_get (LocalVariables|SetNewUnlockedSkins (Variables|/Game/PlayerBlueprints/Blueprints/Saves/GraphicsSaves.GraphicsSaves_C|GetUnlockedSkins _asgraphics_saves)))
    (if (Utilities|Array|ContainsItem (Variables|/Game/PlayerBlueprints/Blueprints/Saves/GraphicsSaves.GraphicsSaves_C|GetUnlockedSkins _asgraphics_saves) SkinToAdd)
      (return false)
      (else
        (Utilities|Array|Add _output_get SkinToAdd)))
    (else
      (bind _returnvalue_3 (SaveGame|CreateSaveGameObject "/Game/PlayerBlueprints/Blueprints/Saves/GraphicsSaves.GraphicsSaves_C"))
      (bind _output_get_2 (LocalVariables|SetNewUnlockedSkins (Variables|/Game/PlayerBlueprints/Blueprints/Saves/GraphicsSaves.GraphicsSaves_C|GetUnlockedSkins _returnvalue_3)))
      (Utilities|Array|Add _output_get_2 SkinToAdd)))
  (bind (_aa_index1 _pp_index1 _fps_index1 _sq_index1 _graphicalindex1) (CallFunction|LoadGraphics false))
  (CallFunction|SaveGraphics _pp_index1 _aa_index1 _sq_index1 _fps_index1 _graphicalindex1 0 (LocalVariables|GetNewUnlockedSkins) 0.0)
  (return true))

(fn SavePlayerLocation
  (params (Location :type Vector))
  (bind _returnvalue (SaveGame|CreateSaveGameObject "/Game/PlayerBlueprints/Blueprints/Saves/LastPlayerLocation.LastPlayerLocation_C"))
  (bind _aslast_player_location (Utilities|Casting|CastToLastPlayerLocation _returnvalue))
  (Variables|/Game/PlayerBlueprints/Blueprints/Saves/LastPlayerLocation.LastPlayerLocation_C|SetLastPlayerLocation _aslast_player_location Location)
  (SaveGame|SaveGametoSlot _aslast_player_location "LastLocation")
  (return))

(fn AdjustSpawnChances
  (Variables|Default|SetCommonChance (Math|Float|Clamp(Float) (- (Variables|Default|GetCommonChance) 2.0) 5e+01 (Variables|Default|GetCommonChance)))
  (Variables|Default|SetRareLowerLimit (Math|Float|Clamp(Float) (- (Variables|Default|GetRareLowerLimit) 2.0) 8e+01 (Variables|Default|GetRareLowerLimit))))

(event EventBeginPlay
  ;[1 1 1] Handle Saves
  (CallFunction|LoadGraphics true)
  (CallFunction|SavePlayerStats 0 0 0.0)
  (bind (_commonitemsunlocked _rareitemsunlocked) (CallFunction|CheckUnlockedItems))
  (CallFunction|SaveUnlocks _commonitemsunlocked _rareitemsunlocked)
  ;[1 1 1] Handle Gameplay Automation
  (CallFunction|StartTimer)
  (CallFunction|SpawnEnemiesTimer)
  (CallFunction|SpawnChests)
  (Class|GameplayStatics|SetBaseSoundMix "/Game/Sounds/Mixes/MasterMix.MasterMix"))

(event Custom|Start%20Timer
  (Utilities|Time|SetTimerbyEvent (delegate Custom|Start%20Timer) 6e+01 true)
  (CallFunction|AdjustSpawnChances)
  (Variables|Default|SetDifficultyMultiplier (+ (Variables|Default|GetDifficultyMultiplier) 0.25))
  (Development|PrintString (Utilities|String|ToString(Float) (Variables|Default|GetDifficultyMultiplier)) true true "(R=0.020839,G=0.000000,B=1.000000,A=1.000000)" 58.0)
  (Development|PrintString "Difficulty Multiplier:" true true "(R=1.000000,G=0.157029,B=0.000000,A=1.000000)" 58.0))

(event Custom|ForceDifficultyIncrease
  (Utilities|FlowControl|Delay 0.2)
  (CallFunction|AdjustSpawnChances)
  (Variables|Default|SetDifficultyMultiplier (+ (Variables|Default|GetDifficultyMultiplier) 0.25))
  (CallFunction|SpawnChests)
  (CallFunction|SpawnEnemies)
  (Development|PrintString (Utilities|String|ToString(Float) (Variables|Default|GetDifficultyMultiplier)) true true "(R=0.020839,G=0.000000,B=1.000000,A=1.000000)" 58.0)
  (Development|PrintString "Difficulty Multiplier:" true true "(R=1.000000,G=0.157029,B=0.000000,A=1.000000)" 58.0))

(event Custom|SpawnEnemiesTimer
  (Utilities|Time|SetTimerbyEvent (delegate Custom|SpawnEnemiesTimer) 3e+01 true)
  (CallFunction|SpawnEnemies))

(event Custom|Dig
  (Default|CallDigi)
  (Utilities|FlowControl|Delay 0.4)
  (Default|CallUndigi))