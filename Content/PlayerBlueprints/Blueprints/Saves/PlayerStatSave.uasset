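; PlayerStatSave is a save object that tracks persistent player statistics: loaders used, deaths, enemies dashed into, enemy kills and a damage record.
; Adder functions increment their counters and immediately save the object itself to the "PlayerStats" slot.
; SetDamageRecord compares run damage against a caller-supplied old record, saves only when it is higher, and returns whether the record was beaten.
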(fn AddtoTotalLoadersUsed
  (params (LoadersUsed :type Integer))
  (Variables|Default|SetTotalLoadersUsed (+ (Variables|Default|GetTotalLoadersUsed) LoadersUsed))
  (SaveGame|SaveGametoSlot self "PlayerStats")
  (return))

(fn AddtoAllTimeDeaths
  (params (Deaths :type Integer))
  (Variables|Default|SetAllTimeDeaths (+ Deaths (Variables|Default|GetAllTimeDeaths)))
  (SaveGame|SaveGametoSlot self "PlayerStats")
  (return))

(fn AddtoEnemiesDashed
  (params (EnemiesDashed :type Integer))
  (Variables|Default|SetEnemiesDashedInto (+ EnemiesDashed (Variables|Default|GetEnemiesDashedInto)))
  (SaveGame|SaveGametoSlot self "PlayerStats")
  (return))

(fn AddtoEnemiesKilledPB
  (params (EnemiesKilledPB :type Integer))
  (Variables|Default|SetEnemiesKilledPB (+ EnemiesKilledPB (Variables|Default|GetEnemiesKilledPB)))
  (SaveGame|SaveGametoSlot self "PlayerStats")
  (return))

(fn SetDamageRecord
  (params (RunDamage :type Float%20%28single-precision%29) (OldDamageRecord :type Float%20%28single-precision%29))
  (if (> RunDamage OldDamageRecord)
    (Variables|Default|SetDamageRecord RunDamage)
    (SaveGame|SaveGametoSlot self "PlayerStats")
    (return true)
    (else
      (return false))))