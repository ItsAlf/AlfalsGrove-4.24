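; Large Stomper enemy that attacks by jumping and creating an area-of-effect damage burst where it lands.
; It overrides Shoot to call Jump, and OnLanded plays a thump and spawns a scaled-up AOE_Damage actor with itself as instigator.
; Projectiles striking its capsule while alive show a green "Blocked!" through the damage-number widget with a sound.
; TriggerRagdoll enables mesh physics, while leftover projectile-firing nodes are unconnected.
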(event OnComponentHit(Capsule)
  (params (HitComponent :type Primitive%20Component%20Object%20Reference) (OtherActor :type Actor%20Object%20Reference) (OtherComp :type Primitive%20Component%20Object%20Reference) (NormalImpulse :type Vector :default "0, 0, 0") (Hit :type Hit%20Result%20Structure%20%28by%20ref%29))
  (Utilities|Casting|CastToBP_Projectile_Parent OtherActor)
  (if (not (Variables|Default|GetIsdead))
    (bind _asdamage_number (Utilities|Casting|CastToDamageNumber (UserInterface|GetUserWidgetObject (Variables|Default|GetDamage%20Number))))
    (Default|PlayAnim _asdamage_number "Blocked!" (Utilities|Struct|MakeSlateColor "(R=0.000000,G=1.000000,B=0.223963,A=1.000000)"))
    (Audio|PlaySoundatLocation "/Game/Sounds/BlockNoise_Cue.BlockNoise_Cue" (Transformation|GetActorLocation) "0, 0, 0" 1.0 1.0 0.0 0 0 0)))

(event Custom|CanShootCooldown
  (Utilities|FlowControl|Delay 0.75))

(event EventShoot
  (Character|Jump))

(event Collision|EventActorBeginOverlap
  (params (OtherActor :type Actor%20Object%20Reference)))

(event EventTick
  (params (DeltaSeconds :type Float%20%28single-precision%29)))

(event EventTriggerRagdoll
  (Class|SkeletalMeshComponent|SetAllBodiesSimulatePhysics (Variables|Character|GetMesh) true))

(event EventOnLanded
  (params (Hit :type Hit%20Result%20Structure%20%28by%20ref%29))
  (bind _location (Collision|BreakHitResult Hit))
  (Audio|PlaySoundatLocation "/Game/Sounds/ThumperLand_Cue.ThumperLand_Cue" _location "0, 0, 0" 1.0 1.0 0.0 0 0 0)
  (Game|SpawnActorfromClass "/Game/Projectiles/AOE_Damage.AOE_Damage_C" (Math|Transform|MakeTransform _location "0, 0, 0" "2.000000,2.000000,2.000000") "Undefined" 0 self))

(fn ConstructionScript
  (|CallParentFunction))