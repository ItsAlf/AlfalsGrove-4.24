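; Turtle enemy that periodically drops damage actors, built on a parent class that supplies base ragdoll and tick behavior.
; A five-second timer, re-armed by HandleDrop, sets Dropping unless dead or staggered.
; NotifyDrop spawns BP_Damage at two drop points, then clears Dropping after a short delay.
; Tick traces downward to smoothly align rotation with the surface normal, and ragdolling enables physics on all mesh bodies.
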(event Custom|HandleDrop
  (Utilities|Time|SetTimerbyEvent (delegate Custom|HandleDrop) 5.0 true)
  (if (not (Variables|Default|GetIsdead))
    (if (not (Variables|Default|GetStaggered))
      (Variables|Default|SetDropping true))))

(event Custom|NotifyDrop
  (for _array_element (Utilities|Array|MakeArray (Variables|Default|GetDropPoint) (Variables|Default|GetDP2))
    (Game|SpawnActorfromClass :Class "/Game/Items/BP_Damage.BP_Damage_C" :SpawnTransform (Math|Transform|MakeTransform (.location (Transformation|GetWorldTransform _array_element)) (.rotation (Transformation|GetWorldTransform _array_element)) "1,1,1") :CollisionHandlingOverride "AdjustIfPossibleButAlwaysSpawn" :Instigator self))
  (Utilities|FlowControl|Delay 0.4)
  (Variables|Default|SetDropping false))

(event EventBeginPlay
  (CallFunction|HandleDrop)
  (|CallParentFunction))

(event Collision|EventActorBeginOverlap
  (params (OtherActor :type Actor%20Object%20Reference)))

(event EventTick
  (params (DeltaSeconds :type Float%20%28single-precision%29))
  (bind _capsulecomponent (Variables|Default|GetCapsuleComponent))
  (bind _returnvalue (Transformation|GetWorldLocation _capsulecomponent))
  (bind (_x _y _z) (Math|Vector|BreakVector _returnvalue))
  (|CallParentFunction DeltaSeconds)
  (bind (_outhit _returnvalue_2) (Collision|LineTraceByChannel _returnvalue (Math|Vector|MakeVector _x _y (- _z 5e+02)) "TraceTypeQuery1" false (Utilities|Array|MakeArray self) "None"))
  (if _returnvalue_2
    (Transformation|SetActorRotation (Math|Interpolation|RInterpTo (Transformation|GetActorRotation) (Math|Rotator|MakeRotfromZX (.ImpactNormal (Collision|BreakHitResult _outhit)) (Transformation|GetActorForwardVector)) 0.5 0.1))))

(event EventTriggerRagdoll
  (|CallParentFunction)
  (Class|SkeletalMeshComponent|SetAllBodiesSimulatePhysics (Variables|Character|GetMesh) true))

(fn ConstructionScript
  (|CallParentFunction))