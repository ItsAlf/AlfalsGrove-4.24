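; BP_Guardian is an enemy that blocks projectiles and damages actors on contact with its weapon.
; Projectile hits on its Box component while alive show a green "Blocked!" popup and play a block sound.
; Gun overlaps apply damage only while attacking, and TriggerRagdoll disables the collision components and simulates mesh physics.
; Tick defers to the parent, and logic aiming ShootPoint at the blackboard's sensed character is left unconnected.
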(event OnComponentHit(Box)
  (params (HitComponent :type Primitive%20Component%20Object%20Reference) (OtherActor :type Actor%20Object%20Reference) (OtherComp :type Primitive%20Component%20Object%20Reference) (NormalImpulse :type Vector :default "0, 0, 0") (Hit :type Hit%20Result%20Structure%20%28by%20ref%29))
  (Utilities|Casting|CastToBP_Projectile_Parent OtherActor)
  (if (not (Variables|Default|GetIsdead))
    (bind _asdamage_number (Utilities|Casting|CastToDamageNumber (UserInterface|GetUserWidgetObject (Variables|Default|GetDamage%20Number))))
    (Default|PlayAnim _asdamage_number "Blocked!" (Utilities|Struct|MakeSlateColor "(R=0.000000,G=1.000000,B=0.223963,A=1.000000)"))
    (Audio|PlaySoundatLocation "/Game/Sounds/BlockNoise_Cue.BlockNoise_Cue" (Transformation|GetActorLocation) "0, 0, 0" 1.0 1.0 0.0 0 0 0)))

(event OnComponentBeginOverlap(Gun)
  (params (OverlappedComponent :type Primitive%20Component%20Object%20Reference) (OtherActor :type Actor%20Object%20Reference) (OtherComp :type Primitive%20Component%20Object%20Reference) (OtherBodyIndex :type Integer) (bFromSweep :type Boolean) (SweepResult :type Hit%20Result%20Structure%20%28by%20ref%29))
  (if (and (Variables|Default|GetAttacking) (!= OtherActor self))
    (Game|Damage|ApplyDamage OtherActor (Variables|Default|GetDamageIDo) (Pawn|GetController) self)))

(event EventBeginPlay
  (|CallParentFunction) ; This node is disabled and will not be called.\nDrag off pins to build functionality.
)

(event Collision|EventActorBeginOverlap
  (params (OtherActor :type Actor%20Object%20Reference)))

(event EventTick
  (params (DeltaSeconds :type Float%20%28single-precision%29))
  (|CallParentFunction DeltaSeconds))

(event EventTriggerRagdoll
  (Collision|SetCollisionEnabled (Variables|Default|GetBox) "NoCollision")
  (Class|SkeletalMeshComponent|SetAllBodiesSimulatePhysics (Variables|Character|GetMesh) true))

(fn ConstructionScript
  (|CallParentFunction))