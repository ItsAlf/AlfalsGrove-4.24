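; BP_EliteArmEnemy is an enemy Blueprint that chases via behavior tree and deals melee damage through capsule overlaps.
; BeginPlay casts its controller to C_Enemy and runs BT_Chase.
; While attacking, either capsule's overlap applies damage to other actors through a shared DoOnce, reset after a short cooldown.
; TriggerRagdoll destroys both capsules and simulates mesh physics; a disconnected branch for turning toward the player never runs.
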(event OnComponentBeginOverlap(Capsule1)
  (params (OverlappedComponent :type Primitive%20Component%20Object%20Reference) (OtherActor :type Actor%20Object%20Reference) (OtherComp :type Primitive%20Component%20Object%20Reference) (OtherBodyIndex :type Integer) (bFromSweep :type Boolean) (SweepResult :type Hit%20Result%20Structure%20%28by%20ref%29))
  (bind _self self)
  (Variables|Default|SetOtherActor OtherActor)
  (if (and (Variables|Default|GetAttacking) (!= (Variables|Default|GetOtherActor) self))
    (Utilities|FlowControl|DoOnce false
      (:Completed
        (CallFunction|DamageCooldown)
        (Game|Damage|ApplyDamage (Variables|Default|GetOtherActor) (Variables|Default|GetDamageIDo) (Pawn|GetController _self) _self)))))

(event OnComponentBeginOverlap(Capsule)
  (params (OverlappedComponent :type Primitive%20Component%20Object%20Reference) (OtherActor :type Actor%20Object%20Reference) (OtherComp :type Primitive%20Component%20Object%20Reference) (OtherBodyIndex :type Integer) (bFromSweep :type Boolean) (SweepResult :type Hit%20Result%20Structure%20%28by%20ref%29))
  (bind _self self)
  (Variables|Default|SetOtherActor OtherActor)
  (if (and (Variables|Default|GetAttacking) (!= (Variables|Default|GetOtherActor) self))
    (Utilities|FlowControl|DoOnce false
      (:Completed
        (CallFunction|DamageCooldown)
        (Game|Damage|ApplyDamage (Variables|Default|GetOtherActor) (Variables|Default|GetDamageIDo) (Pawn|GetController _self) _self)))))

(event Custom|DamageCooldown
  (bind _self self)
  (Utilities|FlowControl|Delay 0.5)
  (Utilities|FlowControl|DoOnce false) ; enters at Reset
)

(event EventBeginPlay
  (|CallParentFunction)
  (bind _asc_enemy (Utilities|Casting|CastToC_Enemy (Pawn|GetController)))
  (bind _output_get (Variables|/Game/Enemies/C_Enemy.C_Enemy_C|SetBehaviorTree _asc_enemy "/Game/Enemies/BT_Chase.BT_Chase"))
  (AI|RunBehaviorTree _asc_enemy _output_get))

(event Collision|EventActorBeginOverlap
  (params (OtherActor :type Actor%20Object%20Reference)))

(event EventTick
  (params (DeltaSeconds :type Float%20%28single-precision%29))
  (|CallParentFunction DeltaSeconds))

(event EventTriggerRagdoll
  (Components|DestroyComponent (Variables|Default|GetCapsule1))
  (Class|SkeletalMeshComponent|SetAllBodiesSimulatePhysics (Variables|Character|GetMesh) true))

(fn ConstructionScript
  (|CallParentFunction))