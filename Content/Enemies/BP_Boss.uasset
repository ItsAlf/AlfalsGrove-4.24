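; BP_Boss is a flying boss enemy that faces the player while bobbing up and down with random sideways drift, switched by a looping timer.
; A second timer's FlipFlop periodically starts DoN-limited attack bursts, tracing down beneath the player to spawn AOE damage and a beam effect from the boss.
; It adds a health bar to the player's HUD, updates it on damage, and on death removes it and changes the music.
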(event Custom|AlternateMovement
  (Utilities|Time|SetTimerbyEvent (delegate Custom|AlternateMovement) 5.0 true)
  (Utilities|FlowControl|FlipFlop
    (:A
      (Variables|Default|SetUp true)
      (Variables|Default|SetDirDiff (Math|Random|RandomIntegerinRange 0 3)))
    (:B
      (Variables|Default|SetUp false)
      (Variables|Default|SetDirDiff (Math|Random|RandomIntegerinRange 0 3)))))

(event Custom|GroundAttack
  (Utilities|Time|SetTimerbyEvent (delegate Custom|GroundAttack) 5.0 true)
  (Utilities|FlowControl|FlipFlop
    (:B
      (Variables|Default|SetShouldIAttack true)
      (Utilities|FlowControl|Sequence
        (:then_0
          (Utilities|FlowControl|DoN (Variables|Default|GetTimesToAttack)) ; enters at Reset
        )
        (:then_1
          (CallFunction|DoAttack))))))

(event Custom|DoAttack
  (Utilities|Time|SetTimerbyEvent (delegate Custom|DoAttack) 0.5 (Variables|Default|GetShouldIAttack))
  (bind _counter (Utilities|FlowControl|DoN (Variables|Default|GetTimesToAttack))
    (:Exit
      (if (>= _counter (Variables|Default|GetTimesToAttack))
        (Variables|Default|SetShouldIAttack false)
        (else
          (bind _asbp_player_character (Utilities|Casting|CastToBP_PlayerCharacter (Game|GetPlayerCharacter 0)))
          (bind (_outhit _returnvalue) (Collision|LineTraceByChannel (Transformation|GetActorLocation _asbp_player_character) (Math|Vector|MakeVector (.X (Math|Vector|BreakVector (Transformation|GetActorLocation _asbp_player_character))) (.Y (Math|Vector|BreakVector (Transformation|GetActorLocation _asbp_player_character))) (- (.Z (Math|Vector|BreakVector (Transformation|GetActorLocation _asbp_player_character))) 6e+03)) "TraceTypeQuery1" false (Utilities|Array|MakeArray _asbp_player_character) "None"))
          (if _returnvalue
            (Game|SpawnActorfromClass "/Game/Projectiles/AOE_Damage.AOE_Damage_C" (Math|Transform|MakeTransform (.Location (Collision|BreakHitResult _outhit)) "0, 0, 0" "1,1,1") "Undefined" 0 self)
            (bind _returnvalue_2 (Effects|SpawnEmitteratLocation "/Game/MyParticles/OldParticles/Exp_FX_P.Exp_FX_P" (.Location (Collision|BreakHitResult _outhit))))
            (Effects|Components|ParticleSystem|SetVectorParameter _returnvalue_2 "Beam_Source" (Transformation|GetActorLocation))
            (Effects|Components|ParticleSystem|SetVectorParameter _returnvalue_2 "Beam_Target" (.Location (Collision|BreakHitResult _outhit)))))))))

(event EventBeginPlay
  (|CallParentFunction)
  (CallFunction|AlternateMovement)
  (CallFunction|GroundAttack)
  (Utilities|FlowControl|Delay 0.0)
  (CallFunction|MakeHPBar))

(event Collision|EventActorBeginOverlap
  (params (OtherActor :type Actor%20Object%20Reference)))

(event EventTick
  (params (DeltaSeconds :type Float%20%28single-precision%29))
  (Transformation|SetWorldRotation (Variables|Default|GetCapsuleComponent) (Math|Rotator|FindLookatRotation (Transformation|GetActorLocation) (Transformation|GetActorLocation (.AsBP%20Player%20Character (Utilities|Casting|CastToBP_PlayerCharacter (Game|GetPlayerCharacter 0))))) false false)
  (if (Variables|Default|GetUp)
    (switch int (Variables|Default|GetDirDiff)
      (:0
        (Pawn|Input|AddMovementInput "0.250000,0.000000,1.000000" 1.0 false))
      (:1
        (Pawn|Input|AddMovementInput "0,0.250000,1.000000" 1.0 false))
      (:2
        (Pawn|Input|AddMovementInput "0.250000,0.250000,1.000000" 1.0 false))
      (:3
        (Pawn|Input|AddMovementInput "0,0.000000,1.000000" 1.0 false)))
    (else
      (switch int (Variables|Default|GetDirDiff)
        (:0
          (Pawn|Input|AddMovementInput "0.250000,0.000000,-1.000000" 1.0 false))
        (:1
          (Pawn|Input|AddMovementInput "0,0.250000,-1.000000" 1.0 false))
        (:2
          (Pawn|Input|AddMovementInput "0.250000,0.250000,-1.000000" 1.0 false))
        (:3
          (Pawn|Input|AddMovementInput "0,0.000000,-1.000000" 1.0 false))))))

(event EventTriggerRagdoll
  (Class|SkeletalMeshComponent|SetAllBodiesSimulatePhysics (Variables|Character|GetMesh) true))

(event EventShoot
  (|CallParentFunction))

(event Game|Damage|EventAnyDamage
  (params (Damage :type Float%20%28single-precision%29) (DamageType :type Damage%20Type%20Object%20Reference) (InstigatedBy :type Controller%20Object%20Reference) (DamageCauser :type Actor%20Object%20Reference))
  (|CallParentFunction Damage DamageType InstigatedBy DamageCauser)
  (Default|TookDamage (Variables|Default|GetMyHP_Bar)))

(event EventDeath
  (Widget|RemovefromParent (Variables|Default|GetMyHP_Bar))
  (bind _asbp_player_character (Utilities|Casting|CastToBP_PlayerCharacter (Game|GetPlayerCharacter 0)))
  (Default|ChangeMusic _asbp_player_character "/Game/Sounds/RL_Reprisal_Cue.RL_Reprisal_Cue")
  (|CallParentFunction))

(fn ConstructionScript
  (|CallParentFunction))

(fn MakeHPBar
  (bind _asbp_player_character (Utilities|Casting|CastToBP_PlayerCharacter (Game|GetPlayerCharacter 0)))
  (bind _returnvalue (UserInterface|CreateWidget "/Game/UI/BossHealthBar.BossHealthBar_C" 0 self))
  (Variables|Default|SetMyHP_Bar _returnvalue)
  (bind _returnvalue_2 (Class|CanvasPanel|AddChildtoCanvas (Variables|/Game/UI/HUD.HUD_C|GetCanvasPanel_0 (Variables|/Game/PlayerBlueprints/Blueprints/BP_PlayerCharacter.BP_PlayerCharacter_C|GetHUD_Ref _asbp_player_character)) _returnvalue))
  (Class|CanvasPanelSlot|SetAutoSize _returnvalue_2 true)
  (Class|CanvasPanelSlot|SetAnchors _returnvalue_2 (Utilities|Struct|MakeAnchors "(X=0.500000,Y=0.000000)" "(X=0.500000,Y=0.000000)"))
  (Class|CanvasPanelSlot|SetPosition _returnvalue_2 "(X=-1000.000000,Y=50.000000)"))