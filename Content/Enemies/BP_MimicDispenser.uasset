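; BP_MimicDispenser is a mimic enemy variant, named for a dispenser, that extends the hide and unhide behavior of its parent class.
; Hide calls the parent and shows the Sphere component without propagating to its children, while Unhide calls the parent and hides Sphere along with its children.
; TriggerRagdoll enables physics simulation on all Mesh bodies, with no parent call.
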(event EventBeginPlay
  (|CallParentFunction) ; This node is disabled and will not be called.\nDrag off pins to build functionality.
)

(event Collision|EventActorBeginOverlap
  (params (OtherActor :type Actor%20Object%20Reference)))

(event EventTick
  (params (DeltaSeconds :type Float%20%28single-precision%29))
  (|CallParentFunction DeltaSeconds) ; This node is disabled and will not be called.\nDrag off pins to build functionality.
)

(event EventTriggerRagdoll
  (Class|SkeletalMeshComponent|SetAllBodiesSimulatePhysics (Variables|Character|GetMesh) true))

(event EventUnhide
  (|CallParentFunction)
  (Rendering|SetVisibility (Variables|Default|GetSphere) false true))

(event EventHide
  (|CallParentFunction)
  (Rendering|SetVisibility (Variables|Default|GetSphere) true false))

(fn ConstructionScript
  (|CallParentFunction))