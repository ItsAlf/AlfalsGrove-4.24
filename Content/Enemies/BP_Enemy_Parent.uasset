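; Base enemy character for a survival mode, scaling health, stagger, damage and heart rewards by game mode difficulty.
; AI blackboard targets drive facing and projectile fire from static mesh components, triggered directly or by notify.
; Damage applies crits, drains a stagger meter that stuns and enables dash executes, and shows flash, sound and number feedback.
; Death triggers a ragdoll hook, drops hearts and random items, and spawns player-enabled explosion or homing effects.
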(event Custom|CheckNameplate
  ;[1 1 1] Handle Nameplate
  (if (Variables|Params|GetShowHP_Bar)
    (Utilities|Time|SetTimerbyEvent (delegate Custom|CheckNameplate) 1.5 true)
    (if (and (> (Transformation|GetDistanceTo (Variables|Default|GetPlayer_Ref)) 1.1e+03) (Rendering|IsVisible (Variables|Default|GetHealthBar)))
      (Rendering|SetVisibility (Variables|Default|GetHealthBar) false false))))

(event Custom|Shoot
  ;[1 1 1] HANDLE SHOOTING
  (if (Variables|Default|GetUsesNotify)
    (Variables|Default|SetShooting true)
    (Variables|Default|SetCanShoot false)
    (CallFunction|ShootCoodlown)
    (elif (Variables|Default|GetCanShoot)
      (Variables|Default|SetShooting true)
      (Variables|Default|SetCanShoot false)
      (CallFunction|ShootCoodlown)
      (Utilities|ShootMacro))))

(event Custom|HandleSpawnAnim
  (Utilities|FlowControl|Delay 1.2)
  (Variables|Default|SetJustSpawned false))

(event Custom|Unhide
  (Variables|Params|SetHiding false))

(event Custom|Hide
  (Variables|Params|SetHiding true))

(event Custom|ShootCoodlown
  ;[1 1 1] HANDLE SHOOTING
  (Utilities|FlowControl|Delay (Variables|Params|GetFireCooldown))
  (Variables|Default|SetCanShoot true))

(event Custom|TriggerRagdoll
  ;[1 1 1] KEEP FOR RAGDOLLING IN OTHER BPS
)

(event Custom|DamageFlash
  (bind _mesh (Variables|Character|GetMesh))
  (bind _returnvalue (Rendering|Material|GetMaterials _mesh))
  ;[1 1 1] Flash when taking damage
  (Utilities|FlowControl|DoOnce false
    (:Completed
      (CallFunction|DamageFlashCooldown)
      (for (_array_element _array_index) _returnvalue
        (Utilities|Array|Add (Variables|Default|GetBaseMaterials) _array_element)
        (Rendering|Material|SetMaterial (Variables|Character|GetMesh) _array_index "/Game/Materials/Projectile_Parent_Mat_Inst.Projectile_Parent_Mat_Inst")
        (bind _asbp_player_character (Utilities|Casting|CastToBP_PlayerCharacter (Game|GetPlayerCharacter 0)))
        (UserInterface|Animation|PlayAnimation (Variables|/Game/PlayerBlueprints/Blueprints/BP_PlayerCharacter.BP_PlayerCharacter_C|GetHUD_Ref _asbp_player_character) (Variables|/Game/UI/HUD.HUD_C|GetHit (Variables|/Game/PlayerBlueprints/Blueprints/BP_PlayerCharacter.BP_PlayerCharacter_C|GetHUD_Ref _asbp_player_character)) 0.0 1 "Forward" 1.0 false))
      (Utilities|FlowControl|Delay 0.25)
      (for (_ _array_index_2) _returnvalue
        (Rendering|Material|SetMaterial (Variables|Character|GetMesh) _array_index_2 (Utilities|Array|Get(acopy) (Variables|Default|GetBaseMaterials) _array_index_2))))))

(event Custom|NotifyShoot
  ;[1 1 1] HANDLE SHOOTING
  (Utilities|ShootMacro))

(event Custom|HandleFlinch
  (Variables|Default|SetFlinch true)
  (Utilities|FlowControl|Delay (Variables|Params|GetFlinchFailsafeTime))
  (Variables|Default|SetFlinch false))

(event Custom|Stagger
  (bind _charactermovement (Variables|Character|GetCharacterMovement))
  ;[1 1 1] Stagger
  (Development|PrintString "Staggered!")
  (AI|Components|Blackboard|SetValueasBool (AI|GetBlackboard (Pawn|GetController)) (Utilities|Name|MakeLiteralName "IsStunned") true)
  (Variables|Default|SetAttacking false)
  (Variables|Damage|SetStaggered true)
  (for _array_element (Variables|Default|GetDynamicMaterials)
    (Rendering|Material|SetScalarParameterValue _array_element "StaggerSpeed" 2.0 :!class /Script/Engine.MaterialInstanceDynamic)
    (bind _returnvalue (Rendering|Material|GetScalarParameterValue _array_element "Emissive" :!class /Script/Engine.MaterialInstanceDynamic))
    (Utilities|Array|Add (Variables|Default|GetEmissivePowers) _returnvalue)
    (Rendering|Material|SetScalarParameterValue _array_element "Emissive" 1.0 :!class /Script/Engine.MaterialInstanceDynamic)
    (Variables|/Script/Engine.CharacterMovementComponent|SetMaxWalkSpeed _charactermovement 0.0))
  (Utilities|FlowControl|Delay 3.0)
  (Variables|Damage|SetStaggered false)
  (for (_array_element_2 _array_index) (Variables|Default|GetDynamicMaterials)
    (Rendering|Material|SetScalarParameterValue _array_element_2 "StaggerSpeed" 0.0 :!class /Script/Engine.MaterialInstanceDynamic)
    (Rendering|Material|SetScalarParameterValue _array_element_2 "Emissive" (Utilities|Array|Get(acopy) (Variables|Default|GetEmissivePowers) _array_index) :!class /Script/Engine.MaterialInstanceDynamic)
    (Variables|/Script/Engine.CharacterMovementComponent|SetMaxWalkSpeed _charactermovement (Variables|Default|GetMyWalkSpeed))))

(event Custom|Damage%20Flash%20Cooldown
  (bind _mesh (Variables|Character|GetMesh))
  (bind _returnvalue (Rendering|Material|GetMaterials _mesh))
  ;[1 1 1] Flash when taking damage
  (Utilities|FlowControl|Delay 0.2)
  (Utilities|FlowControl|DoOnce false) ; enters at Reset
)

(event EventTick
  (params (DeltaSeconds :type Float%20%28single-precision%29))
  (bind _returnvalue (Utilities|Name|MakeLiteralName "SensedCharacter"))
  (bind _returnvalue_2 (Pawn|GetController))
  (bind _returnvalue_3 (Transformation|GetActorTransform))
  (bind _returnvalue_4 (AI|GetBlackboard _returnvalue_2))
  (bind _returnvalue_5 (AI|Components|Blackboard|GetValueasObject _returnvalue_4 _returnvalue))
  (bind _ascharacter (Utilities|Casting|CastToCharacter _returnvalue_5))
  (Utilities|IsValid _ascharacter
    (:Is%20Valid
      (if (or (Variables|Default|GetShooting) (Variables|Default|GetAttacking))
        (if (not (Variables|Damage|GetStaggered))
          (Transformation|SetWorldRotation (Variables|Collision|GetCapsuleComponent) (Math|Rotator|MakeRotator (.roll (.rotation _returnvalue_3)) (.pitch (.rotation _returnvalue_3)) (.yaw (Math|Rotator|FindLookatRotation (Transformation|GetActorLocation) (Transformation|GetActorLocation _ascharacter)))) false false))))))

(fn ConstructionScript)

(fn Die
  (Actor|DestroyActor))

(fn UpdateKills
  (bind _returnvalue (Transformation|GetActorLocation))
  (bind _myheartworth (Variables|Params|GetMyHeartWorth))
  (bind _spawntable (Variables|Params|GetSpawnTable))
  (bind _meshestodrop (Variables|Default|GetMEshesToDrop))
  (bind _returnvalue_2 (/ _myheartworth _meshestodrop))
  (bind _returnvalue_3 (+ (.z _returnvalue) 3e+02))
  (for _index (range 1 (Variables|Default|GetMEshesToDrop))
    (Game|SpawnActorfromClass :Class "/Game/Items/Heart.Heart_C" :SpawnTransform (Math|Transform|MakeTransform (Math|Vector|MakeVector (.x _returnvalue) (.y _returnvalue) _returnvalue_3) "0, 0, 0" "1,1,1") :CollisionHandlingOverride "Undefined" :HeartWorth (select (== _returnvalue_2 0) 1 _returnvalue_2) :Instigator 0))
  (for _index_2 (range 0 (Variables|Params|GetNumberOfItemsToDrop))
    (Game|SpawnActorfromClass :Class (Utilities|Array|Get(acopy) _spawntable (Math|Random|RandomIntegerinRange 0 (- (Utilities|Array|Length _spawntable) 1))) :SpawnTransform (Math|Transform|MakeTransform (Math|Vector|MakeVector (.x _returnvalue) (.y _returnvalue) _returnvalue_3) "0, 0, 0" "1,1,1") :CollisionHandlingOverride "Undefined" :Instigator 0)))

(fn DisplayNameplate
  (if (not (Variables|Default|GetIsdead))
    (if (Variables|Params|GetShowHP_Bar)
      (bind _asenemy_health_bar (Utilities|Casting|CastToEnemyHealthBar (UserInterface|GetUserWidgetObject (Variables|Default|GetHealthBar))))
      (Variables|/Game/UI/EnemyHealthBar.EnemyHealthBar_C|SetEnemy_Ref _asenemy_health_bar self)
      (Rendering|SetVisibility (Variables|Default|GetHealthBar) true false)
      (return))))

(fn CreateDynamicMaterialInstances
  (for (_array_element _array_index) (Rendering|Material|GetMaterials (Variables|Character|GetMesh))
    (bind _returnvalue (Rendering|Material|CreateDynamicMaterialInstance (Variables|Character|GetMesh) _array_index _array_element (Utilities|String|StringToName (Utilities|String|ToString(Integer) _array_index)) :!class /Script/Engine.PrimitiveComponent))
    (Utilities|Array|Add (Variables|Default|GetDynamicMaterials) _returnvalue))
  (return))

(fn HandleIsTargeted
  (bind _targetindicator (Variables|Default|GetTargetIndicator))
  (if (Variables|Default|GetIsdead)
    (Rendering|SetVisibility _targetindicator false false :!label _label)
    (elif (Variables|Default|GetTargeted)
      (Rendering|SetVisibility _targetindicator true false)
      (else
        (goto _label)))))

(fn ShowNumber
  (params (Damage :type Float%20%28single-precision%29) (DamageType :type Damage%20Type%20Class%20Reference))
  (bind _returnvalue (AddComponent|AddWidgetComponent true))
  (Transformation|SetWorldLocation _returnvalue (.location (Transformation|GetWorldTransform (Variables|Default|GetDamage%20Number))) false false)
  (Rendering|SetVisibility _returnvalue true false)
  (Class|WidgetComponent|SetWidgetSpace _returnvalue "Screen")
  (Variables|Default|SetTempNumber _returnvalue)
  (bind _asdamage_number (Utilities|Casting|CastToDamageNumber (UserInterface|GetUserWidgetObject _returnvalue)))
  (Default|PlayAnim _asdamage_number (Utilities|Text|ToText(Integer) (Math|Float|Truncate Damage)) (select (== DamageType "/Game/DamageTypes/CritDamage.CritDamage_C") (Utilities|Struct|MakeSlateColor "(R=1.000000,G=0.000000,B=0.000000,A=1.000000)") (Utilities|Struct|MakeSlateColor "(R=1.000000,G=1.000000,B=1.000000,A=1.000000)")))
  (return))

(fn UpdateHealth
  (params (ChangeAmount :type Float%20%28single-precision%29))
  (Variables|Params|SetCurrentHealth (- (Variables|Params|GetCurrentHealth) ChangeAmount))
  (return))

(event Custom|Death
  (bind _capsulecomponent (Variables|Collision|GetCapsuleComponent))
  (bind _capsulecomponent_2 (Variables|Collision|GetCapsuleComponent))
  (bind _returnvalue (Transformation|GetWorldLocation _capsulecomponent))
  ;[1 1 1] Death
  (Utilities|FlowControl|DoOnce false
    (:Completed
      (Physics|SetSimulatePhysics _capsulecomponent_2 true)
      (Collision|SetCollisionResponsetoChannel _capsulecomponent_2 "ECC_GameTraceChannel2" "ECR_Ignore")
      (Collision|SetCollisionResponsetoChannel _capsulecomponent_2 "ECC_GameTraceChannel3" "ECR_Ignore")
      (Collision|SetCollisionResponsetoChannel _capsulecomponent_2 "ECC_Pawn" "ECR_Ignore")
      (Collision|SetCollisionResponsetoChannel _capsulecomponent_2 "ECC_GameTraceChannel1" "ECR_Ignore")
      (Collision|SetCollisionResponsetoChannel _capsulecomponent_2 "ECC_Visibility" "ECR_Ignore")
      (Collision|SetCollisionResponsetoChannel _capsulecomponent_2 "ECC_Camera" "ECR_Ignore")
      (CallFunction|TriggerRagdoll)
      (Variables|Default|SetIsdead true)
      (CallFunction|UpdateKills)
      (Rendering|SetVisibility (Variables|Default|GetHealthBar) false false)
      (bind _asbp_player_character (Utilities|Casting|CastToBP_PlayerCharacter (Game|GetPlayerCharacter 0)))
      (if (Variables|/Game/PlayerBlueprints/Blueprints/BP_PlayerCharacter.BP_PlayerCharacter_C|GetExplodeOnDeath _asbp_player_character)
        (Game|SpawnActorfromClass "/Game/Projectiles/Explosion.Explosion_C" (Math|Conversions|ToTransform(Vector) (Transformation|GetWorldLocation (Variables|Character|GetMesh))) "Undefined" 0 (Variables|/Game/PlayerBlueprints/Blueprints/BP_PlayerCharacter.BP_PlayerCharacter_C|GetEnemyExplosionSize _asbp_player_character) 0.0 0))
      (if (Variables|/Game/PlayerBlueprints/Blueprints/BP_PlayerCharacter.BP_PlayerCharacter_C|GetHomingOnSpawn _asbp_player_character)
        (Game|SpawnActorfromClass "/Game/Projectiles/HomingSpawnpoint.HomingSpawnpoint_C" (Math|Transform|MakeTransform (Math|Vector|MakeVector (.x _returnvalue) (.y _returnvalue) (+ (.z _returnvalue) 2e+01)) "0, 0, 0" "1,1,1") "Undefined" 0 self))
      (Audio|PlaySoundatLocation (Variables|Params|GetDeathNoise) (Transformation|GetWorldLocation (Variables|Collision|GetCapsuleComponent)) "0, 0, 0" 1.25 0.75 0.0 0 0 0)
      (Variables|/Game/PlayerBlueprints/Blueprints/BP_PlayerCharacter.BP_PlayerCharacter_C|SetTotalKills _asbp_player_character (+ (Variables|/Game/PlayerBlueprints/Blueprints/BP_PlayerCharacter.BP_PlayerCharacter_C|GetTotalKills _asbp_player_character) 1))
      (Utilities|FlowControl|Delay 3.0)
      (CallFunction|Die))))

(event Game|Damage|EventAnyDamage
  (params (Damage :type Float%20%28single-precision%29) (DamageType :type Damage%20Type%20Object%20Reference) (InstigatedBy :type Controller%20Object%20Reference) (DamageCauser :type Actor%20Object%20Reference))
  (AI|Components|Blackboard|SetValueasBool (AI|GetBlackboard (Pawn|GetController)) (Utilities|Name|MakeLiteralName "NoticedSomething") true)
  (Variables|Damage|SetIncomingDamage (* Damage (Variables|Params|GetDamageMultiplier)))
  (Variables|Damage|SetDamageInstigator InstigatedBy)
  (Variables|Damage|SetDamageType DamageType)
  (Variables|Damage|SetDamageCauser DamageCauser)
  (if (and (Variables|Damage|GetStaggered) (== (Utilities|GetClass (Variables|Damage|GetDamageType)) "/Game/DamageTypes/DashDamage.DashDamage_C"))
    ;[1 1 1] Execute
    (Variables|Damage|SetIncomingDamage (Variables|Params|GetMaxHealth))
    (Development|PrintString "EXECUTE")
    (elif (== (Utilities|GetClass (Variables|Damage|GetDamageType)) "/Game/DamageTypes/CritDamage.CritDamage_C")
      (Variables|Damage|SetCritDamage true)
      (Variables|Damage|SetIncomingDamage (* (Variables|Damage|GetIncomingDamage) (Variables|/Game/DamageTypes/CritDamage.CritDamage_C|GetDamageMultiplier (.AsCrit%20Damage (Utilities|Casting|CastToCritDamage (Variables|Damage|GetDamageType))))))
      (else
        (Variables|Damage|SetCritDamage false))))
  (CallFunction|UpdateHealth (Variables|Damage|GetIncomingDamage))
  ;[1 1 1] Damage Feedback
  (bind _asbp_player_character (Utilities|Casting|CastToBP_PlayerCharacter (Variables|Damage|GetDamageCauser))
    (:then
      (CallFunction|DamageFlash)
      (CallFunction|HandleFlinch)
      (Audio|PlaySoundatLocation (Variables|Params|GetDamageNoise) (Transformation|GetActorLocation) "0, 0, 0" 1.0 1.0 0.0 0 0 0)
      (Audio|PlaySound2D (select (Variables|Damage|GetCritDamage) "/Game/Sounds/EnemyTakeCrit_Cue.EnemyTakeCrit_Cue" "/Game/Sounds/HitNoise_Cue.HitNoise_Cue") 1.0 1.0 0.0 0 0)
      (Default|IncreaseDamageDealt _asbp_player_character (Variables|Damage|GetIncomingDamage))
      (bind _asenemy_health_bar (Utilities|Casting|CastToEnemyHealthBar (UserInterface|GetUserWidgetObject (Variables|Default|GetHealthBar)))
        (:then
          (Default|DamageTaken _asenemy_health_bar)
          (CallFunction|ShowNumber (Variables|Damage|GetIncomingDamage) (Utilities|GetClass (Variables|Damage|GetDamageType))))
        (:CastFailed
          _)))
    (:CastFailed
      _))
  (if (<= (Variables|Params|GetCurrentHealth) 0.0)
    (CallFunction|Death)
    (else
      (bind _output_get (Variables|Damage|SetCurrentStaggerHealth (- (Variables|Damage|GetCurrentStaggerHealth) (Variables|Damage|GetIncomingDamage))))
      (if (<= _output_get 0.0)
        (CallFunction|Stagger)
        (Variables|Damage|SetCurrentStaggerHealth (Variables|Params|GetStaggerMaxHealth))))))

(event EventBeginPlay
  (bind _returnvalue (Game|GetGameMode))
  (bind _asgm_survival (Utilities|Casting|CastToGM_Survival _returnvalue))
  (bind _difficultymultiplier (Variables|/Game/PlayerBlueprints/Blueprints/GM_Survival.GM_Survival_C|GetDifficultyMultiplier _asgm_survival))
  ;[0 1 0.224] BEGIN PLAY
  (Variables|/Script/Engine.CharacterMovementComponent|SetMaxWalkSpeed (Variables|Character|GetCharacterMovement) (Variables|Default|GetMyWalkSpeed))
  (CallFunction|HandleSpawnAnim)
  (for _array_element (Actor|GetComponentsByClass "/Script/Engine.StaticMeshComponent")
    (Utilities|Array|Add (Variables|Params|GetArrows) _array_element))
  (CallFunction|CreateDynamicMaterialInstances)
  (Variables|Params|SetDamageIDo (* (Variables|Params|GetDamageIDo) _difficultymultiplier))
  (Variables|Params|SetMaxHealth (* (Variables|Params|GetMaxHealth) _difficultymultiplier))
  (Variables|Params|SetStaggerMaxHealth (* _difficultymultiplier (Variables|Params|GetStaggerMaxHealth)))
  (Variables|Params|SetMyHeartWorth (Math|Float|Truncate (* (* (Variables|Params|GetMyHeartWorth) _difficultymultiplier) (Variables|Default|GetHeartScalingQuotient))))
  (Variables|Params|SetCurrentHealth (Variables|Params|GetMaxHealth))
  (Variables|Damage|SetCurrentStaggerHealth (Variables|Params|GetStaggerMaxHealth))
  (Variables|Default|SetPlayer_Ref (.AsBP%20Player%20Character (Utilities|Casting|CastToBP_PlayerCharacter (Game|GetPlayerCharacter 0))))
  (CallFunction|CheckNameplate)
  (bind _output_get (Variables|Default|SetController_Ref (.AsEnemy%20Controller (Utilities|Casting|CastToEnemy_Controller (Pawn|GetController)))))
  (Variables|/Game/Enemies/Enemy_Controller.Enemy_Controller_C|SetNoticeNoise _output_get (Variables|Params|GetNoticeNoise))
  (Audio|Components|Audio|Play (Variables|Default|GetLoop) 0.0))